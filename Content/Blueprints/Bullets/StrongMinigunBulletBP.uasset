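; StrongMinigunBulletBP is a minigun projectile that bursts on hit and damages robot and brute enemies.
; Its construction script sets the projectile's initial speed from a variable.
; Each hit spawns a small ExplosionBP, then uses actor tags to choose decal and impact particles, skipping decals on NoDecal and Glass surfaces.
; The bullet then destroys itself and subtracts fixed health directly from RobotBP or BruteBP through casts.
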(event `self.ReceiveHit`
  (params (MyComp :type "PrimitiveComponent Object Reference") (Other :type "Actor Object Reference") (OtherComp :type "PrimitiveComponent Object Reference") (bSelfMoved :type Boolean) (HitLocation :type "Vector Structure") (HitNormal :type "Vector Structure") (NormalImpulse :type "Vector Structure") (Hit :type "HitResult Structure (by ref)"))
  (bind _returnvalue (`KismetMathLibrary.Conv_VectorToRotator` HitNormal))
  (`|SpawnActorFromClass` "/Game/FirstPersonBP/AllAssets/Blueprints/ExplosionBP.ExplosionBP_C" (`KismetMathLibrary.MakeTransform` HitLocation (struct) (0.1 0.1 0.1)) "Undefined" "OverrideRootScale")
  (if (`self.ActorHasTag` Other "NoDecal")
    (if (`self.ActorHasTag` Other "Enemy")
      (bind _returnvalue_2 (`GameplayStatics.SpawnEmitterAtLocation` "/Game/StarterContent/Particles/BulletImpact.BulletImpact" HitLocation _returnvalue :!label _label))
      (`SceneComponent.SetRelativeScale3D` _returnvalue_2 (0.5 0.5 0.5)))
    (elif (`self.ActorHasTag` Other "Glass")
      _
      (else
        (`GameplayStatics.SpawnDecalAtLocation` "/Game/FirstPersonBP/AllAssets/Effects/Materials/Weapon/M_Impact_Decal.M_Impact_Decal" (7.0 14.0 14.0) HitLocation _returnvalue 5.0)
        (goto _label))))
  (`self.K2_DestroyActor`)
  (bind _asrobot_bp (cast `/Game/FirstPersonBP/AllAssets/Blueprints/Robots/Robot/RobotBP` Other)
    (:`then`
      (set `/Game/FirstPersonBP/AllAssets/Blueprints/Robots/Robot/RobotBP.RobotHealth` (- (`/Game/FirstPersonBP/AllAssets/Blueprints/Robots/Robot/RobotBP.RobotHealth` _asrobot_bp) 20.0) _asrobot_bp))
    (:`CastFailed`
      (bind _asbrute_bp (cast `/Game/FirstPersonBP/AllAssets/Blueprints/Robots/Brute/BruteBP` Other))
      (set `/Game/FirstPersonBP/AllAssets/Blueprints/Robots/Brute/BruteBP.BruteHealth` (- (`/Game/FirstPersonBP/AllAssets/Blueprints/Robots/Brute/BruteBP.BruteHealth` _asbrute_bp) 20.0) _asbrute_bp))))

(fn `UserConstructionScript`
  (set `ProjectileMovementComponent.InitialSpeed` (`self.ProjectileSpeed`) (`self.Projectile`)))